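; Inventory component that tracks item quantities in a map keyed by item class.
; AddItemToInventory takes the item's class and adds the amount to its stored count.
; RemoveItemFromInventory accepts only BP_ItemsBase subclasses and prints an error for others.
; Removal overwrites the stored count with the amount forced to zero or negative, rather than subtracting from it.
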(fn `AddItemToInventory`
  (params (Item :type "/Game/ItemResources/BP_ItemsBase Object Reference") (Amount :type Integer))
  (bind _returnvalue (`GameplayStatics.GetObjectClass` Item))
  (`BlueprintMapLibrary.Map_Add` (`self.Inventory`) _returnvalue (+ Amount (`BlueprintMapLibrary.Map_Find` (`self.Inventory`) _returnvalue))))

(fn `RemoveItemFromInventory`
  (params (Item :type "/Game/ItemResources/BP_ItemsBase Class Reference") (Amount :type Integer))
  (bind _inventory (`self.Inventory`))
  (if (`KismetMathLibrary.ClassIsChildOf` Item "/Game/ItemResources/BP_ItemsBase.BP_ItemsBase_C")
    (if (< Amount 0)
      (`BlueprintMapLibrary.Map_Add` _inventory Item Amount)
      (else
        (`BlueprintMapLibrary.Map_Add` _inventory Item (* Amount -1))))
    (else
      (`KismetSystemLibrary.PrintString` (`KismetTextLibrary.Conv_TextToString` (`|FormatText` "Item is not child of Item base - {item}" (`KismetSystemLibrary.GetClassDisplayName` Item)))))))
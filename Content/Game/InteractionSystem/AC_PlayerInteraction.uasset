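; Player interaction component that lets its owning Character use BPI_Interactable actors via Enhanced Input.
; Capsule overlaps maintain an in-range list, whose last entry is active and shows a prompt on a runtime-created screen-space widget component.
; IA_Interact handles Press, Hold or Tap per target, using dynamically bound dispatchers for hold timing and progress reset.
; On activation, the character turns toward the interaction point and sends the target its Interact message.
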(event `self.ReceiveBeginPlay`
  ; Enable Character/Childs to use the Interact Component
  (bind _ascharacter (cast `Character` (`self.GetOwner`)))
  (set `self.CharacterRef` _ascharacter)
  (bind _capsulecomponent (`Character.CapsuleComponent` _ascharacter))
  (add `PrimitiveComponent.OnComponentBeginOverlap` _capsulecomponent (`|CreateDelegate` :!event `HandleCapsuleOverlapBegin`))
  (add `PrimitiveComponent.OnComponentEndOverlap` _capsulecomponent (`|CreateDelegate` :!event `HandleCapsuleOverlapEnd`))
  (bind _returnvalue (`|AddComponentByClass` :`self` (`self.GetOwner`) :`Class` "/Script/UMG.WidgetComponent" :`bManualAttachment` true))
  (`WidgetComponent.SetWidgetSpace` _returnvalue "Screen")
  (`WidgetComponent.SetDrawSize` _returnvalue (250.0 30.0))
  (set `self.InteractWidgetComponent` _returnvalue))

(event `HandleCapsuleOverlapBegin`
  (params (OverlappedComponent :type "PrimitiveComponent Object Reference") (OtherActor :type "Actor Object Reference") (OtherComp :type "PrimitiveComponent Object Reference") (OtherBodyIndex :type Integer) (bFromSweep :type Boolean) (SweepResult :type "HitResult Structure (by ref)"))
  ; Add/Remove Interactable actors when going in & out of range
  (if (`KismetSystemLibrary.DoesImplementInterface` OtherActor "/Game/Game/InteractionSystem/BPI_Interactable.BPI_Interactable_C")
    (`KismetArrayLibrary.Array_AddUnique` (`self.InteractablesInRange`) OtherActor)
    (`self.RenderInteractionWidget`)))

(event `EnhancedInput|/Game/Input/Actions/IA_Interact`
  (params (ActionValue :type Boolean) (ElapsedSeconds :type "Float (double-precision)") (TriggeredSeconds :type "Float (double-precision)") (InputAction :type "InputAction Object Reference" :default "/Game/Input/Actions/IA_Interact.IA_Interact"))
  ; Enhanced Input
  (:`Started`
    (`self.InteractBegin`))
  (:`Ongoing`
    (`self.OnInteractPressedOngoing` ElapsedSeconds))
  (:`Canceled`
    (clear `self.OnInteractPressedOngoing` :!label _label)
    (`self.OnInteractEnded`))
  (:`Completed`
    (goto _label)))

(event `HandleCapsuleOverlapEnd`
  (params (OverlappedComponent :type "PrimitiveComponent Object Reference") (OtherActor :type "Actor Object Reference") (OtherComp :type "PrimitiveComponent Object Reference") (OtherBodyIndex :type Integer))
  ; Add/Remove Interactable actors when going in & out of range
  (if (`KismetSystemLibrary.DoesImplementInterface` OtherActor "/Game/Game/InteractionSystem/BPI_Interactable.BPI_Interactable_C")
    (if (== (`self.GetActiveInteractable`) OtherActor)
      (`self.ResetInteractState`))
    (`KismetArrayLibrary.Array_RemoveItem` (`self.InteractablesInRange`) OtherActor)
    (`self.RenderInteractionWidget`)))

(event `InteractTapOngoing`
  ; Tap Interact Logic
  (`GameplayStatics.PlaySound2D` "/Engine/VREditor/Sounds/VR_click2.VR_click2" 1.0 1.0 0.0 null null)
  (`/Engine/EditorBlueprintResources/StandardMacros.IncrementInt` (`self.CurrentTapCount`)
    (:`  `
      (bind _tapcount (message `/Game/Game/InteractionSystem/BPI_Interactable.GetTapCount` (`self.GetActiveInteractable`)))
      (if (<= _tapcount 0)
        (`self.ActivateInteract`)
        (else
          (bind _interactwidgetref (`self.InteractWidgetRef`)
            (:`then`
              (`/Game/Game/InteractionSystem/WBP_InteractDisplay.SetProgressPercent` _interactwidgetref (/ (`self.CurrentTapCount`) _tapcount))
              (if (>= (`self.CurrentTapCount`) _tapcount)
                (`self.ActivateInteract`)))
            (:`else`)))))))

(event `ActivateInteract`
  (bind _characterref (`self.CharacterRef`))
  (bind (_returnvalue_roll _returnvalue_pitch _returnvalue_yaw) (`KismetMathLibrary.BreakRotator` (`KismetMathLibrary.FindLookAtRotation` (`Actor.K2_GetActorLocation` _characterref) (`self.GetInteractLocation`))))
  ; When The Interaction Actually Activates
  (`/Engine/EditorBlueprintResources/StandardMacros.IsValid` (`self.GetActiveInteractable`)
    (:`Is Valid`
      (`Actor.K2_SetActorRotation` _characterref (`KismetMathLibrary.MakeRotator` 0.0 0.0 _returnvalue_yaw) false)
      (message `/Game/Game/InteractionSystem/BPI_Interactable.Interact` (`self.GetActiveInteractable`) (`self.GetOwner`))
      (`self.RenderInteractionWidget`)
      (`self.ResetInteractState`))))

(event `InteractHoldOngoing` :!signature `self.OnInteractPressedOngoing`
  (params (ElapsedSeconds :type "Float (double-precision)"))
  (bind _activeinteractable (`self.GetActiveInteractable`))
  ; Hold Interact Logic
  (`/Engine/EditorBlueprintResources/StandardMacros.IsValid` _activeinteractable
    (:`Is Valid`
      (bind _holdduration (message `/Game/Game/InteractionSystem/BPI_Interactable.GetHoldDuration` _activeinteractable))
      (bind _interactwidgetref (`self.InteractWidgetRef`)
        (:`then`
          (`/Game/Game/InteractionSystem/WBP_InteractDisplay.SetProgressPercent` _interactwidgetref (/ ElapsedSeconds _holdduration)))
        (:`else`
          _))
      (if (> ElapsedSeconds _holdduration)
        (`self.ActivateInteract`)
        (remove `self.OnInteractPressedOngoing` (delegate `InteractHoldOngoing`))))))

(event `InteractBegin`
  (bind _activeinteractable (`self.GetActiveInteractable`))
  ; Which Interact Type Logic
  (`/Engine/EditorBlueprintResources/StandardMacros.IsValid` _activeinteractable
    (:`Is Valid`
      (bind _type (message `/Game/Game/InteractionSystem/BPI_Interactable.GetInteractType` _activeinteractable))
      (switch `/Game/Game/InteractionSystem/E_InteractionType` _type
        (:`NewEnumerator0`
          (`self.ActivateInteract`))
        (:`NewEnumerator1`
          (add `self.OnInteractPressedOngoing` (`|CreateDelegate` :!event `InteractHoldOngoing`))
          (add `self.OnInteractEnded` (delegate `ResetWidgetProgress`)))
        (:`NewEnumerator2`
          (`self.InteractTapOngoing`))))))

(event `ResetWidgetProgress`
  ; Which Interact Type Logic
  (bind _interactwidgetref (`self.InteractWidgetRef`)
    (:`then`
      (`/Game/Game/InteractionSystem/WBP_InteractDisplay.SetProgressPercent` _interactwidgetref 0.0)
      (remove `self.OnInteractEnded` (delegate `ResetWidgetProgress`)))
    (:`else`)))

(fn `GetActiveInteractable`
  (returns (ActiveInteractable :type "Actor Object Reference"))
  (bind _interactablesinrange (`self.InteractablesInRange`))
  (return (`|GetArrayItem` _interactablesinrange (`KismetArrayLibrary.Array_LastIndex` _interactablesinrange))))

(fn `GetInteractLocation`
  (returns (ReturnValue :type "Vector Structure"))
  (bind _activeinteractable (`self.GetActiveInteractable`))
  (bind (_returnvalue_x _returnvalue_y _returnvalue_z) (`KismetMathLibrary.BreakVector` (`Actor.K2_GetActorLocation` _activeinteractable)))
  (`/Engine/EditorBlueprintResources/StandardMacros.IsValid` _activeinteractable
    (:`Is Valid`
      (bind _location (message `/Game/Game/InteractionSystem/BPI_Interactable.GetDisplayLocation` _activeinteractable))
      (return (`KismetMathLibrary.SelectVector` (`KismetMathLibrary.MakeVector` _returnvalue_x _returnvalue_y (- _returnvalue_z 50.0)) _location (`KismetMathLibrary.Vector_IsZero` _location))))))

(fn `RenderInteractionWidget`
  (bind _activeinteractable (`self.GetActiveInteractable`))
  (bind _interactwidgetcomponent (`self.InteractWidgetComponent`))
  (`/Engine/EditorBlueprintResources/StandardMacros.IsValid` _activeinteractable
    (:`Is Valid`
      (bind _type (message `/Game/Game/InteractionSystem/BPI_Interactable.GetInteractType` _activeinteractable))
      (bind _prompt (message `/Game/Game/InteractionSystem/BPI_Interactable.GetInteractPrompt` _activeinteractable))
      (bind _returnvalue (`|CreateWidget` "/Game/Game/InteractionSystem/WBP_InteractDisplay.WBP_InteractDisplay_C" null _type _prompt))
      (set `self.InteractWidgetRef` _returnvalue)
      (`WidgetComponent.SetWidget` _interactwidgetcomponent _returnvalue)
      (`SceneComponent.K2_SetWorldLocation` _interactwidgetcomponent (`self.GetInteractLocation`) false false))
    (:`Is Not Valid`
      ; Hide Widget (after player goes out of range)
      (`WidgetComponent.SetWidget` (`self.InteractWidgetComponent`) null))))

(fn `ResetInteractState`
  (remove `self.OnInteractPressedOngoing` (`|CreateDelegate` :!event `InteractHoldOngoing`))
  (set `self.CurrentTapCount` 0))
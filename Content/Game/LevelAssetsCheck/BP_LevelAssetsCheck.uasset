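; BP_LevelAssetsCheck is an actor whose Box volume reports on the level assets inside it.
; One function sums the overlapping BP_InvasivePlants and BP_RubbishBase actors into a single count.
; Another returns the first overlapping BP_Spawner, or prints an error naming the checker when none is found.
; It runs no logic on its own; its event graph and construction script are empty.
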(fn `Get All Trash and Invasive Plants`
  (returns (Amount :type Integer))
  (bind _box (`self.Box`))
  (return (+ (`KismetArrayLibrary.Array_Length` (`PrimitiveComponent.GetOverlappingActors` _box "/Game/RemovalObjects/InvasivePlants/BP_InvasivePlants.BP_InvasivePlants_C")) (`KismetArrayLibrary.Array_Length` (`PrimitiveComponent.GetOverlappingActors` _box "/Game/RemovalObjects/Rubbish/BP_RubbishBase.BP_RubbishBase_C")))))

(fn `Get Level Spawner`
  (returns (Spawner :type "/Game/Game/Animals_AI_And_Spawning/Spawners/BP_Spawner Object Reference"))
  (bind _output (`|GetArrayItem` (`PrimitiveComponent.GetOverlappingActors` (`self.Box`) "/Game/Game/Animals_AI_And_Spawning/Spawners/BP_Spawner.BP_Spawner_C")))
  (`/Engine/EditorBlueprintResources/StandardMacros.IsValid` _output
    (:`Is Valid`
      (bind _asbp_spawner (cast `/Game/Game/Animals_AI_And_Spawning/Spawners/BP_Spawner` _output))
      (return _asbp_spawner))
    (:`Is Not Valid`
      (`KismetSystemLibrary.PrintString` (`KismetTextLibrary.Conv_TextToString` (`|FormatText` (`KismetSystemLibrary.GetDisplayName` self) "NO SPAWNER WITHIN {self}")) true true (struct :`R` 1.0 :`B` 0.127996 :`A` 1.0) 10.0))))

(fn `UserConstructionScript`)
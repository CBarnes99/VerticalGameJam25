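; AC_Camera is a camera component that takes in-game photos, keeps a rolling photo history and toggles the camera controls widget.
; TakePhoto assigns a new 1080p render target to the given SceneCapture2D, stores it, then captures the scene and returns it.
; UpdateArray drops the oldest photo beyond AmountOfPhotos and fires UpdatedPhotos, which runs before the capture.
; UpdateUI shows or removes the controls widget based on player state.
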(event `self.ReceiveBeginPlay`)

(fn `Take Photo`
  (params (`Scene Capture Target 2D` :type "SceneCaptureComponent2D Object Reference"))
  (returns (`Texture Target` :type "TextureRenderTarget2D Object Reference"))
  (bind _returnvalue (`KismetRenderingLibrary.CreateRenderTarget2D` 1920 1080))
  (bind _output_get (set `SceneCaptureComponent2D.TextureTarget` _returnvalue `Scene Capture Target 2D`))
  (`self.Update Array` _output_get)
  (`SceneCaptureComponent2D.CaptureScene` `Scene Capture Target 2D`)
  (return _output_get))

(fn `Update Array`
  (params (Photo :type "TextureRenderTarget2D Object Reference"))
  (locals (`Amount of Photos` :type Integer :default 6))
  (`KismetArrayLibrary.Array_Add` (`self.Photo Array`) Photo)
  (if (> (`KismetArrayLibrary.Array_Length` (`self.Photo Array`)) (`local.Amount of Photos`))
    (`KismetArrayLibrary.Array_Remove` (`self.Photo Array`)))
  (`self.Updated Photos`))

(fn `Update UI`
  (params (`Player State` :type "/Game/Game/Widgets/selectwheel/E_PlayerState Enum" :default "NewEnumerator0"))
  (if (`|EnumEquality` `Player State` "NewEnumerator1")
    (`UserWidget.AddToViewport` (`self.Camera Contols Widget`) 0)
    (else
      (`Widget.RemoveFromParent` (`self.Camera Contols Widget`)))))
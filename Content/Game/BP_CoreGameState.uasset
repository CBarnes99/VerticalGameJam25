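; Core game state for an environmental cleanup game that tracks progress and rewards a cleared level with an animal.
; On BeginPlay it sets the score to minus the count of rubbish and invasive plant actors, creates the score widget and finds the level's spawner, printing a warning if none exists.
; AddScore counts up toward zero and updates the widget; reaching exactly zero makes the spawner spawn the animal class.
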(event `self.ReceiveBeginPlay`
  (`self.Set Starting Score`)
  (bind _returnvalue (`|CreateWidget` "/Game/Game/Widgets/WBP_Score.WBP_Score_C" null (`self.Score`)))
  (set `self.Score Widget` _returnvalue)
  (`UserWidget.AddToViewport` (`self.Score Widget`) 0)
  (bind _returnvalue_2 (`GameplayStatics.GetActorOfClass` "/Game/Animals/BP_Spawner.BP_Spawner_C"))
  (`/Engine/EditorBlueprintResources/StandardMacros.IsValid` _returnvalue_2
    (:`Is Valid`
      (set `self.Spawner` _returnvalue_2))
    (:`Is Not Valid`
      (`KismetSystemLibrary.PrintString` "NO SPAWNER IN LEVEL" true true (struct :`R` 1.0 :`B` 0.077245 :`A` 1.0) 10.0))))

(fn `Add Score`
  (bind _score (`self.Score`))
  (`/Engine/EditorBlueprintResources/StandardMacros.IncrementInt` _score
    (:`  `
      (`KismetSystemLibrary.PrintString` (`KismetTextLibrary.Conv_TextToString` (`|FormatText` "Score = {score}" _score)))
      (`self.Score Check`)
      (`/Game/Game/Widgets/WBP_Score.Update Score` (`self.Score Widget`) (`self.Score`)))))

(fn `Score Check`
  (if (== (`self.Score`) 0)
    (`self.Spawn Animal`)))

(fn `Set Starting Score`
  (bind _outactors (`GameplayStatics.GetAllActorsOfClass` "/Game/RemovalObjects/Rubbish/BP_RubbishBase.BP_RubbishBase_C"))
  (set `self.Score` (- (`self.Score`) (`KismetArrayLibrary.Array_Length` _outactors)))
  (bind _outactors_2 (`GameplayStatics.GetAllActorsOfClass` "/Game/RemovalObjects/InvasivePlants/BP_InvasivePlants.BP_InvasivePlants_C"))
  (set `self.Score` (- (`self.Score`) (`KismetArrayLibrary.Array_Length` _outactors_2)))
  (`KismetSystemLibrary.PrintString` (`KismetTextLibrary.Conv_TextToString` (`|FormatText` "Starting Score = {score}" (`self.Score`)))))

(fn `Spawn Animal`
  (`/Game/Animals/BP_Spawner.Spawn` (`self.Spawner`) (`self.Animal Class`)))

(fn `UserConstructionScript`)
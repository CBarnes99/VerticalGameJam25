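; BP_AnimalBase is a base animal pawn that continually runs away from the first-person player.
; Two seconds after BeginPlay, Flee starts an AI move to a nearby point directly away from the player at its current height, re-issuing on success or failure.
; Tick starts MovementAnimation's sequence when velocity is non-zero and stops it at rest, using a flag to avoid retriggering.
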(event `self.ReceiveTick`
  (params (DeltaSeconds :type "Float (single-precision)"))
  (if (`KismetMathLibrary.EqualExactly_VectorVector` (`self.GetVelocity`))
    (if (`self.Animation Playing`)
      (`ActorSequenceComponent.StopSequence` (`self.MovementAnimation`))
      (`ActorSequenceComponent.PlaySequence` (`self.MovementAnimation`))
      (`ActorSequenceComponent.StopSequence` (`self.MovementAnimation`))
      (set `self.Animation Playing` false))
    (elif (not (`self.Animation Playing`))
      (`ActorSequenceComponent.PlaySequence` (`self.MovementAnimation`))
      (set `self.Animation Playing` true))))

(event `self.ReceiveBeginPlay`
  (bind _asbp_first_person_character (cast `/Game/FirstPerson/Blueprints/BP_FirstPersonCharacter` (`GameplayStatics.GetPlayerCharacter` 0)))
  (set `self.Char REF` _asbp_first_person_character)
  (`KismetSystemLibrary.Delay` 2.0)
  (`self.Flee`))

(event `Flee`
  (bind _returnvalue (`self.K2_GetActorLocation`))
  (`|AIMoveTo` self (`KismetMathLibrary.MakeVector` (.x (+ _returnvalue (* (`KismetMathLibrary.GetForwardVector` (`KismetMathLibrary.FindLookAtRotation` _returnvalue (`self.K2_GetActorLocation` (`self.Char REF`)))) -100.0))) (.y (+ _returnvalue (* (`KismetMathLibrary.GetForwardVector` (`KismetMathLibrary.FindLookAtRotation` _returnvalue (`self.K2_GetActorLocation` (`self.Char REF`)))) -100.0))) (.z _returnvalue)) null
    (:`OnSuccess`
      _)
    (:`OnFail`
      _))
  (`self.Flee`))

(fn `UserConstructionScript`)
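; BP_CoreGameMode is the game mode that tracks cleanup progress and animal spawning per level.
; On BeginPlay it finds the Level 1 and Level 2 check actors and maps each level number to its trash-and-invasive-plant score target and its spawner.
; UpdateLevelScoreRequired increments the current level and returns that level's target.
; SpawnAnimal triggers the current level's spawner if it is valid.
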(event `self.ReceiveBeginPlay`
  (bind _returnvalue (`GameplayStatics.GetActorOfClass` "/Game/Game/LevelAssetsCheck/BP_Level1Check.BP_Level1Check_C"))
  (bind _output_get (set `self.Level 1 Area` _returnvalue))
  (bind _amount (`/Game/Game/LevelAssetsCheck/BP_LevelAssetsCheck.Get All Trash and Invasive Plants` _output_get))
  (`BlueprintMapLibrary.Map_Add` (`self.Level Score Needed`) 1 _amount)
  (bind _spawner (`/Game/Game/LevelAssetsCheck/BP_LevelAssetsCheck.Get Level Spawner` (`self.Level 1 Area`)))
  (`BlueprintMapLibrary.Map_Add` (`self.Spawners`) 1 _spawner)
  (bind _returnvalue_2 (`GameplayStatics.GetActorOfClass` "/Game/Game/LevelAssetsCheck/BP_Level2Check.BP_Level2Check_C"))
  (bind _output_get_2 (set `self.Level 2 Area` _returnvalue_2))
  (bind _amount_2 (`/Game/Game/LevelAssetsCheck/BP_LevelAssetsCheck.Get All Trash and Invasive Plants` _output_get_2))
  (`BlueprintMapLibrary.Map_Add` (`self.Level Score Needed`) 2 _amount_2)
  (bind _spawner_2 (`/Game/Game/LevelAssetsCheck/BP_LevelAssetsCheck.Get Level Spawner` (`self.Level 2 Area`)))
  (`BlueprintMapLibrary.Map_Add` (`self.Spawners`) 2 _spawner_2))

(fn `Spawn Animal`
  (bind _value (`BlueprintMapLibrary.Map_Find` (`self.Spawners`) (`self.Current Level`)))
  (`/Engine/EditorBlueprintResources/StandardMacros.IsValid` _value
    (:`Is Valid`
      (`/Game/Animals/Spawners/BP_Spawner.Spawn` _value))))

(fn `Update Level Score Required`
  (returns (`Score Amount` :type Integer))
  (bind _output_get (set `self.Current Level` (+ (`self.Current Level`) 1)))
  (return (`BlueprintMapLibrary.Map_Find` (`self.Level Score Needed`) _output_get)))

(fn `UserConstructionScript`)
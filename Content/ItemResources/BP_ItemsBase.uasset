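; BP_ItemsBase is a world item that an interacting first-person character picks up into their inventory.
; Interact adds one unit through the character's ACInventory component, then looks up the item's class in the Inventory map.
; If that entry exists, it prints the stored count and destroys the actor.
; The other interaction functions (prompt, type, location, hold duration, tap count) return only placeholder defaults.
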(event `/Game/Game/InteractionSystem/BPI_Interactable.Interact`
  (params (Interactor :type "Actor Object Reference"))
  (bind _returnvalue (`GameplayStatics.GetObjectClass` self))
  ; Add Item to Inventory
  (`KismetSystemLibrary.PrintString` (`KismetTextLibrary.Conv_TextToString` (`|FormatText` "Interacted with {object}" (`KismetSystemLibrary.GetDisplayName` self))))
  (bind _asbp_first_person_character (cast `/Game/FirstPerson/Blueprints/BP_FirstPersonCharacter` Interactor))
  (bind _ac_inventory (`/Game/FirstPerson/Blueprints/BP_FirstPersonCharacter.AC_Inventory` _asbp_first_person_character))
  (`/Game/Game/AC_Inventory.AddItemToInventory` _ac_inventory self 1)
  (bind (_value _returnvalue_2) (`BlueprintMapLibrary.Map_Find` (`/Game/Game/AC_Inventory.Inventory` _ac_inventory) _returnvalue))
  (if _returnvalue_2
    (`KismetSystemLibrary.PrintString` (`KismetTextLibrary.Conv_TextToString` (`|FormatText` "There are {amount} of {item} in inventory" _value (`KismetSystemLibrary.GetClassDisplayName` _returnvalue))))
    (`self.K2_DestroyActor`)))

(fn `GetDisplayLocation`
  (returns (Location :type "Vector Structure"))
  (return (0.0 0.0 0.0)))

(fn `GetHoldDuration`
  (returns (HoldDuration :type "Float (double-precision)"))
  (return 0.0))

(fn `GetInteractPrompt`
  (returns (Prompt :type Text))
  (return ""))

(fn `GetInteractType`
  (returns (Type :type "/Game/Game/InteractionSystem/E_InteractionType Enum"))
  (return "NewEnumerator0"))

(fn `GetTapCount`
  (returns (TapCount :type Integer))
  (return 0))

(fn `UserConstructionScript`)
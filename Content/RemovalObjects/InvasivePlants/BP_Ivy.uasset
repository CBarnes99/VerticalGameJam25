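; BP_Ivy is an ivy actor among the invasive plant removal objects, with a selectable visual variant.
; Its construction script runs the parent's, then switches on IvyEnum to set the Plant component's first material slot to one of the regular or corner ivy materials.
; The event graph holds only disabled stubs, so this Blueprint adds no runtime logic of its own.
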(fn `UserConstructionScript`
  (`parent.UserConstructionScript`)
  (switch `/Game/RemovalObjects/InvasivePlants/E_Ivy` (`self.Ivy Enum`)
    (:`NewEnumerator0`
      (`PrimitiveComponent.SetMaterial` (`self.Plant`) 0 "/Game/Assets/Grass_Planes/IVY/IvyTexture1_Mat.IvyTexture1_Mat"))
    (:`NewEnumerator1`
      (`PrimitiveComponent.SetMaterial` (`self.Plant`) 0 "/Game/Assets/Grass_Planes/IVY/IvyTexture2_Mat.IvyTexture2_Mat"))
    (:`NewEnumerator2`
      (`PrimitiveComponent.SetMaterial` (`self.Plant`) 0 "/Game/Assets/Grass_Planes/IVY/IvyTexture3_Mat.IvyTexture3_Mat"))
    (:`NewEnumerator3`
      (`PrimitiveComponent.SetMaterial` (`self.Plant`) 0 "/Game/Assets/Grass_Planes/IVY/IvyTexture4_Mat.IvyTexture4_Mat"))
    (:`NewEnumerator4`
      (`PrimitiveComponent.SetMaterial` (`self.Plant`) 0 "/Game/Assets/Grass_Planes/IVY/IvyTexture5_Mat.IvyTexture5_Mat"))
    (:`NewEnumerator5`
      (`PrimitiveComponent.SetMaterial` (`self.Plant`) 0 "/Game/Assets/Grass_Planes/IVY/IvyTexture_Corner1_Mat.IvyTexture_Corner1_Mat"))
    (:`NewEnumerator6`
      (`PrimitiveComponent.SetMaterial` (`self.Plant`) 0 "/Game/Assets/Grass_Planes/IVY/IvyTexture_Corner2_Mat.IvyTexture_Corner2_Mat"))))
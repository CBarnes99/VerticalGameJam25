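; BP_InvasivePlants is an interactable invasive plant that the player removes to earn score.
; It caches BP_CoreGameState on BeginPlay and supplies its plant name as the interact prompt through interaction getters.
; Interact prints a debug message, then, if the first-person character's PlayerState enum matches the first entry, adds score and destroys the plant.
; Destruction plays a sound at world origin rather than the plant's location.
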(event `self.ReceiveBeginPlay`
  (bind _asbp_core_game_state (cast `/Game/Game/BP_CoreGameState` (`GameplayStatics.GetGameState`)))
  (set `self.As BP Core Game State` _asbp_core_game_state))

(event `/Game/Game/InteractionSystem/BPI_Interactable.Interact`
  (params (Interactor :type "Actor Object Reference"))
  (`KismetSystemLibrary.PrintString` (`KismetTextLibrary.Conv_TextToString` (`|FormatText` "Interacted with {object}" (`KismetSystemLibrary.GetDisplayName` self))))
  (bind _asbp_first_person_character (cast `/Game/FirstPerson/Blueprints/BP_FirstPersonCharacter` Interactor))
  (if (`|EnumEquality` (`/Game/FirstPerson/Blueprints/BP_FirstPersonCharacter.Player State` _asbp_first_person_character) "NewEnumerator0")
    (`/Game/Game/BP_CoreGameState.Add Score` (`self.As BP Core Game State`))
    (`self.K2_DestroyActor`)))

(event `self.ReceiveDestroyed`
  (`GameplayStatics.PlaySoundAtLocation` (`AudioComponent.Sound` (`self.SFX`)) (0.0 0.0 0.0) (struct) 1.0 1.0 0.0 null null null null))

(fn `GetDisplayLocation`
  (returns (Location :type "Vector Structure"))
  (return (0.0 0.0 0.0)))

(fn `GetHoldDuration`
  (returns (HoldDuration :type "Float (double-precision)"))
  (return 0.0))

(fn `GetInteractPrompt`
  (returns (Prompt :type Text))
  (return (`self.Plant Name`)))

(fn `GetInteractType`
  (returns (Type :type "/Game/Game/InteractionSystem/E_InteractionType Enum"))
  (return "NewEnumerator0"))

(fn `GetTapCount`
  (returns (TapCount :type Integer))
  (return 0))

(fn `UserConstructionScript`)
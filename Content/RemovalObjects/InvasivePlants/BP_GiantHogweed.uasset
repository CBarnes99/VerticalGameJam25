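; Giant hogweed Blueprint, one of the invasive plant removal objects, with any gameplay behavior left to its parent class.
; The construction script runs the parent's script, then gives the Plant component a random uniform relative scale for size variation.
; The event graph holds only disabled default nodes.
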(fn `UserConstructionScript`
  (`parent.UserConstructionScript`)
  (`SceneComponent.SetRelativeScale3D` (`self.Plant`) (`KismetMathLibrary.Conv_DoubleToVector` (`KismetMathLibrary.RandomFloatInRange` 15.0 30.0))))
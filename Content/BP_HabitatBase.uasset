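; BP_HabitatBase is an interactable habitat build site that starts with an unbuilt material and is completed by handing in required items.
; Each interaction takes one matching item from the player's inventory, decrements the RequiredItems map and refreshes the interaction widget.
; When the map empties, UpdateMaterial swaps to the built material.
; The prompt shows the habitat name plus any outstanding item counts.
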(event `self.ReceiveBeginPlay`
  (`PrimitiveComponent.SetMaterial` (`self.Habitat`) 0 (`self.Unbuilt Material`)))

(event `/Game/Game/InteractionSystem/BPI_Interactable.Interact`
  (params (Interactor :type "Actor Object Reference"))
  (if (> (`BlueprintMapLibrary.Map_Length` (`self.Required Items`)) 0)
    (bind _asbp_first_person_character (cast `/Game/FirstPerson/Blueprints/BP_FirstPersonCharacter` Interactor))
    (bind _keypin (`|MapForEach` (`/Game/Game/AC_Inventory.Inventory` (`/Game/FirstPerson/Blueprints/BP_FirstPersonCharacter.AC_Inventory` _asbp_first_person_character)) :!label _label)
      (:`then`
        (bind (_value _returnvalue) (`BlueprintMapLibrary.Map_Find` (`self.Required Items`) _keypin))
        (if _returnvalue
          (`BlueprintMapLibrary.Map_Add` (`self.Required Items`) _keypin (- _value 1))
          (if (<= (`BlueprintMapLibrary.Map_Find` (`self.Required Items`) _keypin) 0)
            (`BlueprintMapLibrary.Map_Remove` (`self.Required Items`) _keypin))
          (`/Game/Game/AC_Inventory.RemoveItemFromInventory` (`/Game/FirstPerson/Blueprints/BP_FirstPersonCharacter.AC_Inventory` _asbp_first_person_character) _keypin 1)
          (`/Game/Game/InteractionSystem/AC_PlayerInteraction.RenderInteractionWidget` (`/Game/FirstPerson/Blueprints/BP_FirstPersonCharacter.AC_PlayerInteraction` _asbp_first_person_character))
          (`self.Update Material`)
          (goto _label :!via `BreakPin`))))))

(fn `GetDisplayLocation`
  (returns (Location :type "Vector Structure"))
  (bind (_returnvalue_x _returnvalue_y _returnvalue_z) (`KismetMathLibrary.BreakVector` (`self.K2_GetActorLocation` self)))
  (return (`KismetMathLibrary.MakeVector` _returnvalue_x _returnvalue_y (+ _returnvalue_z 50.0))))

(fn `GetHoldDuration`
  (returns (HoldDuration :type "Float (double-precision)"))
  (return 0.0))

(fn `GetInteractPrompt`
  (returns (Prompt :type Text))
  (if (> (`BlueprintMapLibrary.Map_Length` (`self.Required Items`)) 0)
    (bind _all_items (`self.UpdateActorCountText`))
    (return (`|FormatText` "{habitat} \nYou Require: \n{text}" (`self.Habitat Name`) (`KismetTextLibrary.Conv_StringToText` _all_items)))
    (else
      (return (`|FormatText` "{habitat}" (`self.Habitat Name`))))))

(fn `GetInteractType`
  (returns (Type :type "/Game/Game/InteractionSystem/E_InteractionType Enum"))
  (return "NewEnumerator0"))

(fn `GetTapCount`
  (returns (TapCount :type Integer))
  (return 0))

(fn `Update Material`
  (if (<= (`BlueprintMapLibrary.Map_Length` (`self.Required Items`)) 0)
    (`PrimitiveComponent.SetMaterial` (`self.Habitat`) 0 (`self.Built Material`))))

(fn `UpdateActorCountText`
  (returns (`All Items` :type String))
  (locals (DisplayString :type String))
  (bind (_keypin _valuepin) (`|MapForEach` (`self.Required Items`))
    (:`then`
      (set `local.DisplayString` (`KismetStringLibrary.Concat_StrStr` (`local.DisplayString`) (`KismetTextLibrary.Conv_TextToString` (`|FormatText` "{item name}: Count:{Amount} \n" (`KismetSystemLibrary.GetClassDisplayName` _keypin) _valuepin)))))
    (:`CompletedPin`
      (return (`local.DisplayString`)))))

(fn `UserConstructionScript`)
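; Actor placement component that lets a player preview, position, rotate and then place an actor of a given class.
; StartPlacement spawns a collision-free preview, which externally called updates move to Visibility line-trace hits along a supplied direction and rotate in yaw.
; Confirm spawns the real actor at the preview's transform and destroys the preview, while cancel just removes it.
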(fn `CancelPlacement`
  ; Cancels the placement and destorys the preview actor
  (`/Engine/EditorBlueprintResources/StandardMacros.IsValid` (`self.PreviewActor`)
    (:`Is Valid`
      (`Actor.K2_DestroyActor` (`self.PreviewActor`))
      (set `self.bIsPlacing` false)
      (set `self.ActorClass` null))))

(fn `ConfirmPlacement`
  ; Spawns the actor you want to spawn in the location of the preview actor
  (if (and (`KismetSystemLibrary.IsValidClass` (`self.ActorClass`)) (`KismetSystemLibrary.IsValid` (`self.PreviewActor`)))
    (`|SpawnActorFromClass` (`self.ActorClass`) (`Actor.GetTransform` (`self.PreviewActor`)) "Undefined" "MultiplyWithRoot" null null)
    (`Actor.K2_DestroyActor` (`self.PreviewActor`))
    (set `self.bIsPlacing` false)
    (set `self.ActorClass` null)))

(fn `RotatePlacement`
  (params (Direction :type "Float (double-precision)"))
  (bind (_returnvalue_roll _returnvalue_pitch _returnvalue_yaw) (`KismetMathLibrary.BreakRotator` (`Actor.K2_GetActorRotation` (`self.PreviewActor`))))
  ; Rotates the actor on the Z axis
  (`Actor.K2_SetActorRotation` (`self.PreviewActor`) (`KismetMathLibrary.MakeRotator` 0.0 0.0 (+ (* Direction 1.0) _returnvalue_yaw)) false))

(fn `StartPlacement`
  (params (`Actor Class` :type "Actor Class Reference"))
  (bind _previewactor (`self.PreviewActor`))
  ; Initially Spawns the preview actor
  (set `self.ActorClass` `Actor Class`)
  (`/Engine/EditorBlueprintResources/StandardMacros.IsValid` _previewactor
    (:`Is Valid`
      (`Actor.K2_DestroyActor` _previewactor))
    (:`Is Not Valid`
      _))
  (bind _returnvalue (`|SpawnActorFromClass` (`self.ActorClass`) (`KismetMathLibrary.MakeTransform` (0.0 0.0 0.0)) "Undefined" "MultiplyWithRoot" null null))
  (bind _output_get (set `self.PreviewActor` _returnvalue))
  (`Actor.SetActorEnableCollision` _output_get false)
  (set `self.bIsPlacing` true))

(fn `UpdatePlacementLocation`
  (params (`Trace Start Location` :type "Vector Structure") (`Forward Vector` :type "Vector Structure"))
  ; Updates the location of the preview actor
  (bind (_outhit _returnvalue) (`KismetSystemLibrary.LineTraceSingle` `Trace Start Location` (+ `Trace Start Location` (* `Forward Vector` (`self.TraceDistance`))) "TraceTypeQuery1" false (`|MakeArray` (`self.PreviewActor`)) "ForDuration" true (struct :`R` 1.0 :`A` 1.0) (struct :`G` 1.0 :`A` 1.0) 0.2))
  (if _returnvalue
    (`Actor.K2_SetActorLocation` (`self.PreviewActor`) (`.Location` (`GameplayStatics.BreakHitResult` _outhit)) false false)))
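; BP_Rocks is a level design rock prop whose shape is chosen from five variants.
; The Construction Script switches on the RockType value and assigns the matching rock static mesh to the Rock component.
; The event graph holds only disabled default events, so the actor has no runtime logic.
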(fn `UserConstructionScript`
  (switch `/Game/LevelDesign/Enums/E_RockTypes` (`self.Rock Type`)
    (:`NewEnumerator0`
      (`StaticMeshComponent.SetStaticMesh` (`self.Rock`) "/Game/Assets/Rocks/SM_Rock_1.SM_Rock_1"))
    (:`NewEnumerator1`
      (`StaticMeshComponent.SetStaticMesh` (`self.Rock`) "/Game/Assets/Rocks/SM_Rock_2.SM_Rock_2"))
    (:`NewEnumerator2`
      (`StaticMeshComponent.SetStaticMesh` (`self.Rock`) "/Game/Assets/Rocks/SM_Rock_3.SM_Rock_3"))
    (:`NewEnumerator3`
      (`StaticMeshComponent.SetStaticMesh` (`self.Rock`) "/Game/Assets/Rocks/SM_Rock_4.SM_Rock_4"))
    (:`NewEnumerator4`
      (`StaticMeshComponent.SetStaticMesh` (`self.Rock`) "/Game/Assets/Rocks/SM_Rock_5.SM_Rock_5"))))
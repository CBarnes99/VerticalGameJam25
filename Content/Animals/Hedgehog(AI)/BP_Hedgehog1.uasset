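; Hedgehog AI that roams around its spawn point and reacts to seen pawns with a flee move.
; Roaming loops AI moves to random reachable points in a radius, with random pauses between them.
; PawnSensing triggers Flee, which changes walk speed and moves FleeDistance along the look-at direction toward the pawn, then restores speed and resumes roaming.
; Flee checks a Fleeing flag that this graph only ever clears.
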(event `self.ReceiveBeginPlay`
  (set `self.Spawn Location` (`self.K2_GetActorLocation`))
  (`KismetSystemLibrary.Delay` (`self.Roam Interval Min`))
  (`self.Go to Random Location`))

(event `Go to Random Location`
  (`AITask_MoveTo.AIMoveTo` (`AIBlueprintHelperLibrary.GetAIController` self) (`NavigationSystemV1.K2_GetRandomReachablePointInRadius` (`self.Spawn Location`) (`self.Roam Range`) null null) null
    (:`OnRequestFailed`
      _)
    (:`OnMoveFinished`
      _))
  (`KismetSystemLibrary.Delay` (`KismetMathLibrary.RandomFloatInRange` (`self.Roam Interval Min`) (`self.Roam Interval Max`)))
  (`self.Go to Random Location`))

(event `Flee`
  (params (Pawn :type "Pawn Object Reference"))
  (bind _returnvalue (`self.K2_GetActorLocation`))
  (if (not (`self.Fleeing?`))
    (set `CharacterMovementComponent.MaxWalkSpeed` (`self.Flee Walk Speed`) (`self.CharacterMovement`))
    (`AITask_MoveTo.AIMoveTo` (`AIBlueprintHelperLibrary.GetAIController` self) (+ _returnvalue (* (`KismetMathLibrary.GetForwardVector` (`KismetMathLibrary.FindLookAtRotation` _returnvalue (`self.K2_GetActorLocation` Pawn))) (`self.Flee Distance`))) null
      (:`OnRequestFailed`
        _)
      (:`OnMoveFinished`
        _))
    (set `self.Fleeing?` false)
    (set `CharacterMovementComponent.MaxWalkSpeed` (`self.Normal Walk Speed`) (`self.CharacterMovement`))
    (`self.Go to Random Location`)))

(event `self.PawnSensing.OnSeePawn`
  (params (Pawn :type "Pawn Object Reference"))
  (`self.Flee` Pawn))

(fn `UserConstructionScript`)